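; BP_Door is a double sliding door that opens while all of its linked floor buttons are activated.
; On BeginPlay it stores both panels' initial positions and binds to each button's pressed-changed event.
; Each change rechecks every button and plays or reverses a Timeline.
; The Timeline lerps the two panels apart along their relative X axis, so the door closes again when any button deactivates.
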(event Custom|CloseDoor
  (bind _iniposrightdoor (Variables|Default|GetIniPosRightDoor))
  (bind _iniposleftdoor (Variables|Default|GetIniPosLeftDoor))
  (bind _newtrack_0 (Timeline|Timeline Reverse)
    (:Update
      (Transformation|SetRelativeLocation (Variables|Default|GetLeftDoor) (Math|Vector|Lerp(Vector) _iniposleftdoor (- _iniposleftdoor "80.000000,0.000000,0.000000") _newtrack_0) false false)
      (Transformation|SetRelativeLocation (Variables|Default|GetRightDoor) (Math|Vector|Lerp(Vector) _iniposrightdoor (+ _iniposrightdoor "80.000000,0.000000,0.000000") _newtrack_0) false false))))

(event Custom|OpenDoor
  (bind _iniposrightdoor (Variables|Default|GetIniPosRightDoor))
  (bind _iniposleftdoor (Variables|Default|GetIniPosLeftDoor))
  (bind _newtrack_0 (Timeline|Timeline Play)
    (:Update
      (Transformation|SetRelativeLocation (Variables|Default|GetLeftDoor) (Math|Vector|Lerp(Vector) _iniposleftdoor (- _iniposleftdoor "80.000000,0.000000,0.000000") _newtrack_0) false false)
      (Transformation|SetRelativeLocation (Variables|Default|GetRightDoor) (Math|Vector|Lerp(Vector) _iniposrightdoor (+ _iniposrightdoor "80.000000,0.000000,0.000000") _newtrack_0) false false))))

(event Custom|CheckButtons
  (Variables|Default|SetAllPressed true)
  (for _array_element (Variables|Default|GetFloorButtons)
    (if (not (Variables|/Game/00_Examen_UNIR/BP_FloorButton.BP_FloorButton_C|GetButtonActivated _array_element))
      (Variables|Default|SetAllPressed false)))
  (if (Variables|Default|GetAllPressed)
    (CallFunction|OpenDoor)
    (else
      (CallFunction|CloseDoor))))

(event EventBeginPlay
  (Variables|Default|SetIniPosRightDoor (Variables|/Script/Engine.SceneComponent|GetRelativeLocation (Variables|Default|GetRightDoor)))
  (Variables|Default|SetIniPosLeftDoor (Variables|/Script/Engine.SceneComponent|GetRelativeLocation (Variables|Default|GetLeftDoor)))
  (for _array_element (Variables|Default|GetFloorButtons)
    (EventDispatchers|BindEventtoOnPressedChanged _array_element (delegate Custom|CheckButtons))))

(fn ConstructionScript)