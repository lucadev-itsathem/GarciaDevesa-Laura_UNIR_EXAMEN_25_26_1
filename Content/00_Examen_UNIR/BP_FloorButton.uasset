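; BP_FloorButton is a floor button that the player toggles with E, likely to open and close a door.
; Its Box overlap enables input and changes the button material while BP_ThirdPersonCharacter is inside, reverting both on exit.
; Each press flips ButtonActivated, swaps the Lights emissive material and runs CallDoor, which fires the OnPressedChanged dispatcher.
; An interface-based message to DoorActor is left unconnected and never runs.
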(event OnComponentBeginOverlap(Box)
  (params (OverlappedComponent :type Primitive%20Component%20Object%20Reference) (OtherActor :type Actor%20Object%20Reference) (OtherComp :type Primitive%20Component%20Object%20Reference) (OtherBodyIndex :type Integer) (bFromSweep :type Boolean) (SweepResult :type Hit%20Result%20Structure%20%28by%20ref%29))
  (Utilities|Casting|CastToBP_ThirdPersonCharacter OtherActor)
  (Variables|Default|SetPlayerIsInside true)
  (Input|EnableInput (Game|GetPlayerController 0))
  (Rendering|Material|SetMaterial (Variables|Default|GetButton) 1 "/Game/00_Examen_UNIR/M_Color1.M_Color1"))

(event OnComponentEndOverlap(Box)
  (params (OverlappedComponent :type Primitive%20Component%20Object%20Reference) (OtherActor :type Actor%20Object%20Reference) (OtherComp :type Primitive%20Component%20Object%20Reference) (OtherBodyIndex :type Integer))
  (Utilities|Casting|CastToBP_ThirdPersonCharacter OtherActor)
  (Variables|Default|SetPlayerIsInside false)
  (Input|DisableInput (Game|GetPlayerController 0))
  (Rendering|Material|SetMaterial (Variables|Default|GetButton) 1 "/Game/LowPolyAssets/Materials/M_Color.M_Color"))

(event Custom|CallDoor
  (params (Open :type Boolean))
  (Default|CallOnPressedChanged))

(event EventBeginPlay
  (Rendering|Material|SetMaterial (Variables|Default|GetLights) 0 "/Game/LowPolyAssets/Materials/M_Emission.M_Emission"))

(event Collision|EventActorBeginOverlap
  (params (OtherActor :type Actor%20Object%20Reference)))

(event EventTick
  (params (DeltaSeconds :type Float%20%28single-precision%29)))

(event Input|KeyboardEvents|E
  (params (Key :type Key%20Structure :default "None"))
  (:Pressed
    (bind _output_get (Variables|Default|SetButtonActivated (not (Variables|Default|GetButtonActivated))))
    (if _output_get
      (Rendering|Material|SetMaterial (Variables|Default|GetLights) 0 "/Game/00_Examen_UNIR/M_Emission1.M_Emission1")
      (CallFunction|CallDoor true)
      (else
        (Rendering|Material|SetMaterial (Variables|Default|GetLights) 0 "/Game/LowPolyAssets/Materials/M_Emission.M_Emission")
        (CallFunction|CallDoor false)))))

(fn ConstructionScript)